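; Lightning actor that produces recurring strikes with a double screen flash at random intervals of several seconds.
; From BeginPlay it loops, activating the Lightning component for the first flash and pulsing the PostProcess volume's manual exposure compensation for both.
; Each pulse replaces the volume's whole settings struct, restoring only the exposure compensation saved at start.
; Unconnected leftovers hold a directional light flicker and an automatic volume lookup.
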(event `self.ReceiveBeginPlay`
  (set `self.Original Exposure Compensation` (`.AutoExposureBias` (break `PostProcessSettings` (`PostProcessVolume.Settings` (`self.PostProcess`)))))
  (`KismetSystemLibrary.Delay` (`KismetMathLibrary.RandomFloatInRange` 5.0 10.0) :!label _label)
  (`ActorComponent.Activate` (`self.Lightning`) false)
  (set `PostProcessVolume.Settings` (make `PostProcessSettings` :`AutoExposureMethod` "AEM_Manual" :`AutoExposureBias` 11.0) (`self.PostProcess`))
  (`KismetSystemLibrary.Delay` 0.2)
  (set `PostProcessVolume.Settings` (make `PostProcessSettings` :`AutoExposureMethod` "AEM_Manual" :`AutoExposureBias` (`self.Original Exposure Compensation`)) (`self.PostProcess`))
  (`ActorComponent.Deactivate` (`self.Lightning`))
  (`KismetSystemLibrary.Delay` 0.2)
  (set `PostProcessVolume.Settings` (make `PostProcessSettings` :`AutoExposureMethod` "AEM_Manual" :`AutoExposureBias` 11.0) (`self.PostProcess`))
  (`KismetSystemLibrary.Delay` 0.2)
  (set `PostProcessVolume.Settings` (make `PostProcessSettings` :`AutoExposureMethod` "AEM_Manual" :`AutoExposureBias` (`self.Original Exposure Compensation`)) (`self.PostProcess`))
  (goto _label))

(fn `UserConstructionScript`)